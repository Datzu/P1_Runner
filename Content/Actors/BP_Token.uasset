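; BP_Token is a moving obstacle actor that quits the game on any actor overlap and awards points when destroyed.
; Each tick, Move shifts its StaticMesh component in world space along the normalized Direction at MoveVelocity, scaled by delta time, without sweeping.
; BeginPlay sets its life span and caches the BP_GMB game mode, whose UpdatePoints receives PointsGained on Destroyed.
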(event EventBeginPlay
  ;[1 1 1] Starting the actor
  (Actor|SetLifeSpan (Variables|Default|GetLifeSpan))
  (bind _asbp_gmb (Utilities|Casting|CastToBP_GMB (Game|GetGameMode)))
  (Variables|Default|SetGMB _asbp_gmb))

(event Collision|EventActorBeginOverlap
  (params (OtherActor :type Actor%20Object%20Reference))
  ;[1 1 1] Finishing the game
  (Game|QuitGame 0 "Quit" false))

(event EventTick
  (params (DeltaSeconds :type Float%20%28single-precision%29))
  ;[1 1 1] Move every tick
  (CallFunction|Move DeltaSeconds))

(event EventDestroyed
  ;[1 1 1] Detroying the actor when the time is up
  (Default|UpdatePoints (Variables|Default|GetGMB) (Variables|Default|GetPointsGained)))

(fn ConstructionScript)

(fn Move
  (params (deltaTime :type Float%20%28double-precision%29))
  (bind _staticmesh (Variables|Default|GetStaticMesh))
  ;[1 1 1] Calc the next position on the world and set it
  (Transformation|SetWorldLocation _staticmesh (+ (* (* deltaTime (Variables|Default|GetMove%20Velocity)) (Math|Vector|Normalize (Variables|Default|GetDirection))) (Transformation|GetWorldLocation _staticmesh)) false false))