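; Timed spawner actor that repeatedly creates an ObjectToSpawn instance in randomly chosen lanes along the world Y axis.
; A looping timer set on BeginPlay calls SpawnObject, which keeps the root's X, Z, rotation and scale and gives each instance a ten-second life span.
; CalcPos picks Y from Pos0 or Pos1 by a three-way random roll, whose third outcome assigns no new value.
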(event Custom|SpawnActor
  (CallFunction|SpawnObject))

(event EventBeginPlay
  (Utilities|Time|SetTimerbyEvent (delegate Custom|SpawnActor) (Variables|Default|GetSpawnTime) true))

(fn ConstructionScript)

(fn SpawnObject
  (bind _defaultsceneroot (Variables|Default|GetDefaultSceneRoot))
  (bind _returnvalue (Transformation|GetWorldTransform _defaultsceneroot))
  (bind (_location _rotation _scale) (Math|Transform|BreakTransform _returnvalue))
  (bind _calculatedposition (CallFunction|CalcPos _location))
  (bind _returnvalue_2 (Game|SpawnActorfromClass (Variables|Default|GetObjectToSpawn) (Math|Transform|MakeTransform _calculatedposition _rotation _scale) "Undefined" 0 0))
  (Actor|SetLifeSpan _returnvalue_2 1e+01))

(fn CalcPos
  (params (InitialPosition :type Vector))
  (bind (_x _y _z) (Math|Vector|BreakVector InitialPosition))
  (LocalVariables|SetSelectedPosition (Math|Random|RandomIntegerinRange 0 2))
  ;[1 1 1] Conditionals from left or right
  (if (== 0 (LocalVariables|GetSelectedPosition))
    ;[1 1 1] Set the values of the position
    (bind _output_get (LocalVariables|SetCalculatedPos (LocalVariables|GetPos0)))
    (elif (== 1 (LocalVariables|GetSelectedPosition))
      (bind _output_get_2 (LocalVariables|SetCalculatedPos (LocalVariables|GetPos1)))))
  (return (Math|Vector|MakeVector _x (Math|Conversions|ToFloat(Integer) _output_get) _z)))