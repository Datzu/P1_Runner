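; BP_Token is a token actor that moves in a straight line along its Direction and reports what it overlaps.
; Tick calls Move, which offsets the StaticMesh world location by normalized Direction scaled by MoveVelocity and delta time, without sweeping.
; On actor overlap it only prints the other actor's name, apparently as debug output.
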(event EventBeginPlay)

(event Collision|EventActorBeginOverlap
  (params (OtherActor :type Actor%20Object%20Reference))
  (Development|PrintString (Utilities|GetDisplayName OtherActor)))

(event EventTick
  (params (DeltaSeconds :type Float%20%28single-precision%29))
  (CallFunction|Move DeltaSeconds))

(fn ConstructionScript)

(fn Move
  (params (deltaTime :type Float%20%28double-precision%29))
  (bind _staticmesh (Variables|Default|GetStaticMesh))
  (Transformation|SetWorldLocation _staticmesh (+ (* (* deltaTime (Variables|Default|GetMove%20Velocity)) (Math|Vector|Normalize (Variables|Default|GetDirection))) (Transformation|GetWorldLocation _staticmesh)) false false))