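; Player character that steps sideways on Left and Right input presses, starting from a fixed position teleported to in the construction script.
; MoveLeft and MoveRight get a target from CalcPos, which shifts world Y by MovePos and clamps it on the side of travel to that same distance from zero.
; MoveTo then sets the static mesh's world location directly, without sweep, rather than moving the actor.
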(event Input|ActionEvents|InputActionLeft
  (params (Key :type Key%20Structure :default "None"))
  ;[1 1 1] Left action
  (:Pressed
    (CallFunction|MoveLeft)))

(event Input|ActionEvents|InputActionRight
  (params (Key :type Key%20Structure :default "None"))
  ;[1 1 1] Right action
  (:Pressed
    (CallFunction|MoveRight)))

(fn ConstructionScript
  ;[1 1 1] We have to teleport to initial pos, because potatoes :D
  (Transformation|Teleport "420.000000, 0,20.000000" "0, 0, 0"))

(fn Moveto
  (params (Position :type Vector))
  ;[1 1 1] Get the mesh and refresh pos in world
  (Transformation|SetWorldLocation (Variables|Default|GetStaticMesh) Position false false))

(fn GetWorldLocation
  (return (Transformation|GetWorldLocation (Variables|Default|GetStaticMesh))))

(fn CalcPos
  (params (Direction :type Text))
  (bind _movepos (LocalVariables|GetMovePos))
  (if (Utilities|Enum|Equal(Enum) (Class|KismetTextLibrary|TexttoLower Direction) (LocalVariables|GetLEFT))
    ;[1 1 1] Left calc
    (bind _location (CallFunction|GetWorldLocation))
    (return (Math|Vector|MakeVector (.X (Math|Vector|BreakVector _location)) (Math|Float|Min(Float) (+ (.Y (Math|Vector|BreakVector _location)) _movepos) _movepos) (.Z (Math|Vector|BreakVector _location))))
    (elif (Utilities|Enum|Equal(Enum) (Class|KismetTextLibrary|TexttoLower Direction) (LocalVariables|GetRIGHT))
      ;[1 1 1] Right calc
      (bind _location_2 (CallFunction|GetWorldLocation))
      (return (Math|Vector|MakeVector (.X (Math|Vector|BreakVector _location_2)) (Math|Float|Max(Float) (* _movepos -1.0) (- (.Y (Math|Vector|BreakVector _location_2)) _movepos)) (.Z (Math|Vector|BreakVector _location_2))))
      (else
        ;[1 1 1] No value
        (Development|PrintString "ERROR - Direction not implemented")))))

(fn MoveLeft
  (bind _location (CallFunction|CalcPos (LocalVariables|GetDirection)))
  (CallFunction|Moveto _location))

(fn MoveRight
  (bind _location (CallFunction|CalcPos (LocalVariables|GetDirection)))
  (CallFunction|Moveto _location))